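; BP_PlayerPawn is the player pawn, a sphere steered by Enhanced Input in swept steps and 90-degree turns, which holds one usable power.
; AddPower_Event stores the power; using it levitates the sphere, slows CrusherObject or quits the game.
; A timer flags levitation or slow for reset.
; Tick then retries the swept drop to default height until unblocked, restoring crusher speed and re-enabling power use.
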(event `EnhancedInput|/Game/Input/IA_MoveForward`
  (params (ActionValue :type Boolean) (ElapsedSeconds :type "Float (double-precision)") (TriggeredSeconds :type "Float (double-precision)") (InputAction :type "InputAction Object Reference" :default "/Game/Input/IA_MoveForward.IA_MoveForward"))
  (bind _sphere (`self.Sphere`))
  ; Movement
  (:`Triggered`
    (`SceneComponent.K2_AddRelativeLocation` _sphere (* (`SceneComponent.GetForwardVector` _sphere) (`self.Speed`)) true false)))

(event `self.ReceiveBeginPlay`
  (bind _returnvalue (`SceneComponent.GetRelativeTransform` (`self.Sphere`)))
  (`|ExecutionSequence`
    (:`then_0`
      ; Set levitation params (can't be done in construction, because relative transform is needed)
      (bind _output_get (set `self.DefaultHeight` (.z (.location _returnvalue))))
      (set `self.LevitatedHeight` (+ _output_get (`self.LevitationChange`)))
      (set `self.StartPosition` _returnvalue))
    (:`then_1`
      ; AddMappingContext On BeginPlay
      (bind _asplayer_controller (cast `PlayerController` (`self.GetController`)))
      (`EnhancedInputSubsystemInterface.AddMappingContext` (pcsubsystem `EnhancedInputLocalPlayerSubsystem` _asplayer_controller) "/Game/Input/IMC_Player.IMC_Player" 0 (struct)))))

(event `EnhancedInput|/Game/Input/IA_MoveBack`
  (params (ActionValue :type Boolean) (ElapsedSeconds :type "Float (double-precision)") (TriggeredSeconds :type "Float (double-precision)") (InputAction :type "InputAction Object Reference" :default "/Game/Input/IA_MoveBack.IA_MoveBack"))
  (bind _sphere (`self.Sphere`))
  ; Movement
  (:`Triggered`
    (`SceneComponent.K2_AddRelativeLocation` _sphere (* (`SceneComponent.GetForwardVector` _sphere) (* (`self.Speed`) -1.0)) true false)))

(event `EnhancedInput|/Game/Input/IA_RotateRight`
  (params (ActionValue :type Boolean) (ElapsedSeconds :type "Float (double-precision)") (TriggeredSeconds :type "Float (double-precision)") (InputAction :type "InputAction Object Reference" :default "/Game/Input/IA_RotateRight.IA_RotateRight"))
  ; Rotation
  (:`Triggered`
    (`SceneComponent.K2_AddRelativeRotation` (`self.Sphere`) (struct :`Yaw` 90.0) false false)))

(event `EnhancedInput|/Game/Input/IA_RotateLeft`
  (params (ActionValue :type Boolean) (ElapsedSeconds :type "Float (double-precision)") (TriggeredSeconds :type "Float (double-precision)") (InputAction :type "InputAction Object Reference" :default "/Game/Input/IA_RotateLeft.IA_RotateLeft"))
  ; Rotation
  (:`Triggered`
    (`SceneComponent.K2_AddRelativeRotation` (`self.Sphere`) (struct :`Yaw` -90.0) false false)))

(event `AddPower_Event`
  (params (PowerObtained :type "/Game/E_PowerType Enum" :default "NewEnumerator0"))
  ; Add a new power
  (bind _output_get (set `self.PowerHeld` PowerObtained))
  (`KismetSystemLibrary.PrintText` (`|GenericToText` _output_get)))

(event `EnhancedInput|/Game/Input/IA_UsePower`
  (params (ActionValue :type Boolean) (ElapsedSeconds :type "Float (double-precision)") (TriggeredSeconds :type "Float (double-precision)") (InputAction :type "InputAction Object Reference" :default "/Game/Input/IA_UsePower.IA_UsePower"))
  ; Power functionality
  (:`Triggered`
    (if (`self.PowerActivated`)
      (`KismetSystemLibrary.PrintString` "AbilityAlreadyInProgress")
      (else
        (switch `/Game/E_PowerType` (`self.PowerHeld`)
          (:`NewEnumerator0`
            (`self.SetLocationHeight` (`self.LevitatedHeight`))
            (set `self.PowerActivated` true :!label _label)
            (`KismetSystemLibrary.K2_SetTimerDelegate` (delegate `EndAbility`) (`self.PowerDuration`)))
          (:`NewEnumerator1`
            (`/Game/AC_Crusher.GoSlower_Event` (`self.CrusherObject`))
            (goto _label))
          (:`NewEnumerator3`
            (`KismetSystemLibrary.QuitGame` null "Quit")))))))

(event `EndAbility`
  ; Power functionality
  (set `self.ShouldRestartPower` true))

(event `self.ReceiveTick`
  (params (DeltaSeconds :type "Float (single-precision)"))
  (if (`self.ShouldRestartPower`)
    ; Power effects restart
    (bind _wasblocked (`self.SetLocationHeight` (`self.DefaultHeight`)))
    (if _wasblocked
      (set `self.ShouldRestartPower` true)
      (else
        (`/Game/AC_Crusher.GoDefaultSpeed_Event` (`self.CrusherObject`))
        (set `self.ShouldRestartPower` false)
        (set `self.PowerActivated` false)))))

(fn `SetLocationHeight`
  (params (Height :type "Float (double-precision)"))
  (returns (WasBlocked :type Boolean))
  (bind _returnvalue (`KismetMathLibrary.MakeVector` (.x (.location (`SceneComponent.GetRelativeTransform` (`self.Sphere`)))) (.y (.location (`SceneComponent.GetRelativeTransform` (`self.Sphere`)))) Height))
  (bind _sweephitresult (`SceneComponent.K2_SetRelativeLocation` (`self.Sphere`) _returnvalue true false))
  (`KismetSystemLibrary.PrintText` (`KismetTextLibrary.Conv_VectorToText` _returnvalue))
  (return (`GameplayStatics.BreakHitResult` _sweephitresult)))

(fn `UserConstructionScript`)