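; Crusher hazard actor that teleports any overlapping BP_PlayerPawn back to its start position.
; Tick moves the Cube component up and down at the current speed, reversing when its relative height reaches the upper or lower bound.
; Two events switch between slower and default speed, and the construction script initializes the speed to default.
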(event `GoSlower_Event`
  (set `self.CurrentSpeed` (`self.SlowerSpeed`)))

(event `GoDefaultSpeed_Event`
  (set `self.CurrentSpeed` (`self.DefaultSpeed`)))

(event `self.ReceiveBeginPlay`)

(event `self.ReceiveTick`
  (params (DeltaSeconds :type "Float (single-precision)"))
  (bind _z (.z (.location (`SceneComponent.GetRelativeTransform` (`self.Cube`)))))
  ; Crusher movement
  (if (`self.GoingUp`)
    (`SceneComponent.K2_AddRelativeLocation` (`self.Cube`) (* (`KismetMathLibrary.Vector_Up`) (`self.CurrentSpeed`) DeltaSeconds) false false)
    (else
      (`SceneComponent.K2_AddRelativeLocation` (`self.Cube`) (* (`KismetMathLibrary.Vector_Down`) (`self.CurrentSpeed`) DeltaSeconds) false false)))
  (if (>= _z (`self.UpperBound`))
    (set `self.GoingUp` false)
    (elif (<= _z (`self.LowerBound`))
      (set `self.GoingUp` true))))

(event `self.ReceiveActorBeginOverlap`
  (params (OtherActor :type "Actor Object Reference"))
  ; PlayerReset
  (bind _asbp_player_pawn (cast `/Game/BP_PlayerPawn` OtherActor))
  (`self.K2_SetActorTransform` _asbp_player_pawn (`/Game/BP_PlayerPawn.StartPosition` _asbp_player_pawn) false true))

(fn `UserConstructionScript`
  (set `self.CurrentSpeed` (`self.DefaultSpeed`)))